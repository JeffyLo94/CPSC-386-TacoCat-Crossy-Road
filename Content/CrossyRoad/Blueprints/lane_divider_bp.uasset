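; Lane divider actor for Crossy Road that awards the chicken a lane-crossed point when it overlaps the actor.
; On BeginPlay it adds a row of ten evenly spaced Grass mesh components along Y, made invisible with a Transparent material.
; These meshes have overlap events on but collision set to NoCollision.
; ActorBeginOverlap casts to CR_Chicken and calls AddLaneCrossedPoint, ignoring other actors.
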(event `self.ReceiveBeginPlay`
  (for _index (range 10)
    (bind _returnvalue (`AddComponent|NODE_AddStaticMeshComponent-0` :`RelativeTransform` (`KismetMathLibrary.MakeTransform` (`KismetMathLibrary.MakeVector` 0.0 (* _index 100.0)) (struct :`Yaw` 270.0 :`Roll` 180.0) (100.0 100.0 100.0))))
    (`StaticMeshComponent.SetStaticMesh` _returnvalue "/Game/CrossyRoad/Meshes/grass.grass")
    (`PrimitiveComponent.SetMaterial` _returnvalue 0 "/Game/CrossyRoad/Materials/Transparent.Transparent")
    (`PrimitiveComponent.SetMaterial` _returnvalue 1 "/Game/CrossyRoad/Materials/Transparent.Transparent")
    (`PrimitiveComponent.SetCollisionEnabled` _returnvalue "NoCollision")
    (set `PrimitiveComponent.bGenerateOverlapEvents` true _returnvalue)))

(event `self.ReceiveActorBeginOverlap`
  (params (OtherActor :type "Actor Object Reference"))
  (bind _ascr_chicken (cast `/Game/CrossyRoad/Blueprints/CR_Chicken` OtherActor))
  (`/Game/CrossyRoad/Blueprints/CR_Chicken.addLaneCrossedPoint` _ascr_chicken))

(fn `UserConstructionScript`)