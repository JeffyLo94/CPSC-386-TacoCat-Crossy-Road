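; Lane spawner for a Crossy Road-style game that builds a strip of river lanes when play begins.
; BeginPlay loops along X at fixed spacing from the actor's location, calling SpawnRiverLogs to place a river and an offset log.
; Helpers for highways with cars and for grass exist but are not run.
; The lilypad helper has no class set, and the tree-rock helper spawns only grass.
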(event `self.ReceiveBeginPlay`
  (for _index (range 11)
    (`self.SpawnRiverLogs` (+ (`SceneComponent.K2_GetComponentLocation` (`self.DefaultSceneRoot`)) (`KismetMathLibrary.MakeVector` (* _index 100.0))))))

(fn `SpawnGrass`
  (params (SpawnLocation :type "Vector Structure"))
  (`|SpawnActorFromClass` "/Game/CrossyRoad/Blueprints/grass_bp.grass_bp_C" (`KismetMathLibrary.MakeTransform` SpawnLocation) "Undefined" "OverrideRootScale" null null))

(fn `SpawnGrassTreeRock`
  (params (SpawnLocation :type "Vector Structure"))
  (`|SpawnActorFromClass` "/Game/CrossyRoad/Blueprints/grass_bp.grass_bp_C" (`KismetMathLibrary.MakeTransform` SpawnLocation) "Undefined" "OverrideRootScale" null null))

(fn `SpawnHighwayMulti`
  (params (SpawnLocation :type "Vector Structure"))
  (`|SpawnActorFromClass` "/Game/CrossyRoad/Blueprints/highway_multi_bp.highway_multi_bp_C" (`KismetMathLibrary.MakeTransform` SpawnLocation) "Undefined" "OverrideRootScale" null null)
  (`|SpawnActorFromClass` "/Game/CrossyRoad/Blueprints/car_bp.car_bp_C" (`KismetMathLibrary.MakeTransform` (+ SpawnLocation (50.0 -900.0 10.0))) "Undefined" "OverrideRootScale" null null))

(fn `SpawnHighwaySingle`
  (params (SpawnLocation :type "Vector Structure"))
  (`|SpawnActorFromClass` "/Game/CrossyRoad/Blueprints/highway_single_bp.highway_single_bp_C" (`KismetMathLibrary.MakeTransform` SpawnLocation) "Undefined" "OverrideRootScale" null null)
  (`|SpawnActorFromClass` "/Game/CrossyRoad/Blueprints/car_bp.car_bp_C" (`KismetMathLibrary.MakeTransform` (+ SpawnLocation (50.0 -900.0 10.0))) "Undefined" "OverrideRootScale" null null))

(fn `SpawnRiverLilypads`
  (params (SpawnLocation :type "Vector Structure"))
  (`|SpawnActorFromClass` "/Game/CrossyRoad/Blueprints/river_bp.river_bp_C" (`KismetMathLibrary.MakeTransform` SpawnLocation) "Undefined" "OverrideRootScale" null null))

(fn `SpawnRiverLogs`
  (params (SpawnLocation :type "Vector Structure"))
  (`|SpawnActorFromClass` "/Game/CrossyRoad/Blueprints/river_bp.river_bp_C" (`KismetMathLibrary.MakeTransform` SpawnLocation) "Undefined" "OverrideRootScale" null null)
  (`|SpawnActorFromClass` "/Game/CrossyRoad/Blueprints/log_bp.log_bp_C" (`KismetMathLibrary.MakeTransform` (+ SpawnLocation (50.0 -900.0 10.0))) "Undefined" "OverrideRootScale" null null))

(fn `UserConstructionScript`)