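; Log actor for a Crossy Road style game that drifts along the Y axis in an endless loop.
; On BeginPlay it adds a medium log mesh with its material, rotates and scales the actor, and picks a random speed.
; Each Tick it moves by that speed without delta-time scaling, so motion depends on frame rate.
; Leaving the fixed Y bounds snaps it back near the negative end.
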(event `self.ReceiveBeginPlay`
  (bind _returnvalue (`AddComponent|NODE_AddStaticMeshComponent-0`))
  (`StaticMeshComponent.SetStaticMesh` _returnvalue "/Game/CrossyRoad/Meshes/log_medium.log_medium")
  (`self.K2_SetActorTransform` (`KismetMathLibrary.MakeTransform` (`SceneComponent.K2_GetComponentLocation` (`self.DefaultSceneRoot`)) (struct :`Yaw` 90.0 :`Roll` 90.0) (50.0 50.0 50.0)))
  (`PrimitiveComponent.SetMaterial` _returnvalue 0 "/Game/CrossyRoad/Materials/log_material.log_material")
  (set `self.speed` (`KismetMathLibrary.RandomFloatInRange` 3.0 7.0)))

(event `self.ReceiveTick`
  (params (DeltaSeconds :type "Float (single-precision)"))
  (bind (_returnvalue_x _returnvalue_y) (`KismetMathLibrary.BreakVector` (`self.K2_GetActorLocation`)))
  (bind (_returnvalue_x_2 _returnvalue_y_2 _returnvalue_z) (`KismetMathLibrary.BreakVector` (`self.K2_GetActorLocation`)))
  (bind (_returnvalue_x_3 _returnvalue_y_3 _returnvalue_z_2) (`KismetMathLibrary.BreakVector` (`self.K2_GetActorLocation`)))
  (`self.K2_SetActorLocation` (`KismetMathLibrary.MakeVector` _returnvalue_x_3 (+ _returnvalue_y_3 (`self.speed`)) _returnvalue_z_2))
  (if (or (< _returnvalue_y -1000.0) (> _returnvalue_y 1000.0))
    (`self.K2_SetActorLocation` (`KismetMathLibrary.MakeVector` _returnvalue_x_2 -900.0 _returnvalue_z))))

(fn `UserConstructionScript`)