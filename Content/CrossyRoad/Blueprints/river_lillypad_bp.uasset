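; River lane actor for a Crossy Road-style game that builds a strip of water with lilypads on it.
; On BeginPlay it adds ten River mesh components at even steps along Y, rotated, scaled up and given the Palette material.
; Each segment also spawns a Lillypad_bp actor slightly offset in X and raised above it.
; A switch on a constant before the spawn has empty branches, and the construction script is empty.
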(event `self.ReceiveBeginPlay`
  (for _index (range 10)
    (bind _returnvalue (`AddComponent|NODE_AddStaticMeshComponent-0` :`RelativeTransform` (`KismetMathLibrary.MakeTransform` (`KismetMathLibrary.MakeVector` 0.0 (* (`KismetMathLibrary.Conv_IntToDouble` _index) 100.0)) (struct :`Roll` 90.0) (100.0 100.0 100.0))))
    (`StaticMeshComponent.SetStaticMesh` _returnvalue "/Game/CrossyRoad/Meshes/river.river")
    (`PrimitiveComponent.SetMaterial` _returnvalue 0 "/Game/CrossyRoad/Materials/palette.palette")
    (`PrimitiveComponent.SetMaterial` _returnvalue 1 "/Game/CrossyRoad/Materials/palette.palette")
    (switch `int` 0
      (:`Default`
        _)
      (:`0`
        _))
    (bind (_returnvalue_x _returnvalue_y _returnvalue_z) (`KismetMathLibrary.BreakVector` (`SceneComponent.K2_GetComponentLocation` _returnvalue)))
    (`|SpawnActorFromClass` "/Game/CrossyRoad/Blueprints/lillypad_bp.lillypad_bp_C" (`KismetMathLibrary.MakeTransform` (`KismetMathLibrary.MakeVector` (+ _returnvalue_x 50.0) _returnvalue_y (+ _returnvalue_z 10.0))) "Undefined" "OverrideRootScale" null null)))

(fn `UserConstructionScript`)