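; Car obstacle actor for a Crossy Road style game that drives endlessly along the world Y axis.
; On BeginPlay it adds a static mesh component with one of four random car or truck models, applies the palette material, rotates and scales the actor, and rolls a random speed.
; Tick adds that speed to Y each frame, without delta-time scaling, and resets Y near the negative end once it leaves the lane bounds.
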(event `self.ReceiveBeginPlay`
  (bind _returnvalue (`AddComponent|NODE_AddStaticMeshComponent-0`))
  (`StaticMeshComponent.SetStaticMesh` _returnvalue (select `int` (`KismetMathLibrary.RandomIntegerInRange` 0 3) :`0` "/Game/CrossyRoad/Meshes/car_purple.car_purple" :`1` "/Game/CrossyRoad/Meshes/crossyroad_blue_car.crossyroad_blue_car" :`2` "/Game/CrossyRoad/Meshes/crossyroad_green_car.crossyroad_green_car" :`3` "/Game/CrossyRoad/Meshes/truck_red.truck_red" :!type "StaticMesh Object Reference"))
  (`self.K2_SetActorTransform` (`KismetMathLibrary.MakeTransform` (`SceneComponent.K2_GetComponentLocation` (`self.DefaultSceneRoot`)) (struct :`Roll` 90.0) (50.0 50.0 50.0)))
  (`PrimitiveComponent.SetMaterial` _returnvalue 0 "/Game/CrossyRoad/Materials/palette.palette")
  (set `self.speed` (`KismetMathLibrary.RandomFloatInRange` 1.0 3.0)))

(event `self.ReceiveTick`
  (params (DeltaSeconds :type "Float (single-precision)"))
  (bind (_returnvalue_x _returnvalue_y) (`KismetMathLibrary.BreakVector` (`self.K2_GetActorLocation`)))
  (bind (_returnvalue_x_2 _returnvalue_y_2 _returnvalue_z) (`KismetMathLibrary.BreakVector` (`self.K2_GetActorLocation`)))
  (bind (_returnvalue_x_3 _returnvalue_y_3 _returnvalue_z_2) (`KismetMathLibrary.BreakVector` (`self.K2_GetActorLocation`)))
  (`self.K2_SetActorLocation` (`KismetMathLibrary.MakeVector` _returnvalue_x_3 (+ _returnvalue_y_3 (`self.speed`)) _returnvalue_z_2))
  (if (or (< _returnvalue_y -1000.0) (> _returnvalue_y 1000.0))
    (`self.K2_SetActorLocation` (`KismetMathLibrary.MakeVector` _returnvalue_x_2 -900.0 _returnvalue_z))))

(fn `UserConstructionScript`)